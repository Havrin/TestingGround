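; Tile actor for infinite terrain, with a gate, trigger volumes and an arrow marking its attach point.
; Player entry into LockingVolume opens the green gate; leaving it turns the gate red and solid, then asks InfiniteTerrainGameMode to spawn a tile.
; Player overlap with DestroyVolume destroys the tile, and GetAttachLocation exposes the arrow's world transform.
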(event `self.ReceiveBeginPlay`)

(event `self.LockingVolume.OnComponentBeginOverlap`
  (params (OverlappedComponent :type "PrimitiveComponent Object Reference") (OtherActor :type "Actor Object Reference") (OtherComp :type "PrimitiveComponent Object Reference") (OtherBodyIndex :type Integer) (bFromSweep :type Boolean) (SweepResult :type "HitResult Structure (by ref)"))
  (`self.Is Player` OtherActor)
  (`self.Unlock`))

(event `self.LockingVolume.OnComponentEndOverlap`
  (params (OverlappedComponent :type "PrimitiveComponent Object Reference") (OtherActor :type "Actor Object Reference") (OtherComp :type "PrimitiveComponent Object Reference") (OtherBodyIndex :type Integer))
  (`self.Is Player` OtherActor)
  (`self.Lock`)
  (bind _asinfinite_terrain_game_mode (cast `/Game/Dynamic/InfiniteTerrainGameMode` (`GameplayStatics.GetGameMode`)))
  (`/Game/Dynamic/InfiniteTerrainGameMode.Spawn Tile` _asinfinite_terrain_game_mode))

(event `self.DestroyVolume.OnComponentBeginOverlap`
  (params (OverlappedComponent :type "PrimitiveComponent Object Reference") (OtherActor :type "Actor Object Reference") (OtherComp :type "PrimitiveComponent Object Reference") (OtherBodyIndex :type Integer) (bFromSweep :type Boolean) (SweepResult :type "HitResult Structure (by ref)"))
  (`self.Is Player` OtherActor)
  (`self.K2_DestroyActor`))

(fn `Get Attach Location`
  (returns (`Attach Transform` :type "Transform Structure"))
  (return (`SceneComponent.K2_GetComponentToWorld` (`self.Arrow`))))

(fn `Lock`
  (`PrimitiveComponent.SetCollisionEnabled` (`self.Gate`) "QueryAndPhysics")
  (`PrimitiveComponent.SetMaterial` (`self.Gate`) 0 "/Game/Dynamic/Terrain/RedBarrier.RedBarrier"))

(fn `Unlock`
  (`PrimitiveComponent.SetCollisionEnabled` (`self.Gate`) "NoCollision")
  (`PrimitiveComponent.SetMaterial` (`self.Gate`) 0 "/Game/Dynamic/Terrain/GreenBarrier.GreenBarrier"))

(fn `UserConstructionScript`)