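; BP_Tile is an infinite-terrain tile that scatters containers, rocks, canisters, boxes and sandbags on BeginPlay through PlaceActors calls.
; The player entering LockingVolume unlocks the gate, while leaving it locks the gate and asks InfiniteTerrainGameMode to spawn another tile.
; Gate state toggles collision and a green or red material, and GetAttachLocation exposes the Arrow's world transform.
; The tile destroys itself when the player overlaps DestroyVolume.
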(event `self.ReceiveBeginPlay`
  (`self.PlaceActors` "/Game/Dynamic/Terrain/Props/BP_Container.BP_Container_C" 1 3 1.0 1.0 400.0)
  (`self.PlaceActors` "/Game/Dynamic/Terrain/Props/BP_Rock1.BP_Rock1_C" 2 5 1.0 5.0 150.0)
  (`self.PlaceActors` "/Game/Dynamic/Terrain/Props/BP_Rock2.BP_Rock2_C" 1 3 1.0 5.0 250.0)
  (`self.PlaceActors` "/Game/Dynamic/Terrain/Props/BP_Rock3.BP_Rock3_C" 2 7 1.0 5.0 250.0)
  (`self.PlaceActors` "/Game/Dynamic/Terrain/Props/BP_SingleCanister.BP_SingleCanister_C" 1 3 1.0 1.0 50.0)
  (`self.PlaceActors` "/Game/Dynamic/Terrain/Props/BP_MultipleCanisters.BP_MultipleCanisters_C" 2 4 1.0 1.0 100.0)
  (`self.PlaceActors` "/Game/Dynamic/Terrain/Props/BP_Box.BP_Box_C" 3 6 1.0 1.0 100.0)
  (`self.PlaceActors` "/Game/Dynamic/Terrain/Props/BP_Sandbags.BP_Sandbags_C" 5 15 1.0 1.0 250.0))

(event `self.LockingVolume.OnComponentBeginOverlap`
  (params (OverlappedComponent :type "PrimitiveComponent Object Reference") (OtherActor :type "Actor Object Reference") (OtherComp :type "PrimitiveComponent Object Reference") (OtherBodyIndex :type Integer) (bFromSweep :type Boolean) (SweepResult :type "HitResult Structure (by ref)"))
  (`self.Is Player` OtherActor)
  (`self.Unlock`))

(event `self.LockingVolume.OnComponentEndOverlap`
  (params (OverlappedComponent :type "PrimitiveComponent Object Reference") (OtherActor :type "Actor Object Reference") (OtherComp :type "PrimitiveComponent Object Reference") (OtherBodyIndex :type Integer))
  (`self.Is Player` OtherActor)
  (`self.Lock`)
  (bind _asinfinite_terrain_game_mode (cast `/Game/Dynamic/InfiniteTerrainGameMode` (`GameplayStatics.GetGameMode`)))
  (`/Game/Dynamic/InfiniteTerrainGameMode.Spawn Tile` _asinfinite_terrain_game_mode))

(event `self.DestroyVolume.OnComponentBeginOverlap`
  (params (OverlappedComponent :type "PrimitiveComponent Object Reference") (OtherActor :type "Actor Object Reference") (OtherComp :type "PrimitiveComponent Object Reference") (OtherBodyIndex :type Integer) (bFromSweep :type Boolean) (SweepResult :type "HitResult Structure (by ref)"))
  (`self.Is Player` OtherActor)
  (`self.K2_DestroyActor`))

(fn `Get Attach Location`
  (returns (`Attach Transform` :type "Transform Structure"))
  (return (`SceneComponent.K2_GetComponentToWorld` (`self.Arrow`))))

(fn `Lock`
  (`PrimitiveComponent.SetCollisionEnabled` (`self.Gate`) "QueryAndPhysics")
  (`PrimitiveComponent.SetMaterial` (`self.Gate`) 0 "/Game/Dynamic/Terrain/MI_Barrier_Red.MI_Barrier_Red"))

(fn `Unlock`
  (`PrimitiveComponent.SetCollisionEnabled` (`self.Gate`) "NoCollision")
  (`PrimitiveComponent.SetMaterial` (`self.Gate`) 0 "/Game/Dynamic/Terrain/MI_Barrier_Green.MI_Barrier_Green"))

(fn `UserConstructionScript`)