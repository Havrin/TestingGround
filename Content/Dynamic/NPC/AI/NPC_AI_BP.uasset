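; NPC_AI_BP is an AI controller for patrolling guards that starts the GuardBehaviour tree with the PatrolData blackboard.
; Perception updates on actors without the "Enemy" tag switch the possessed PatrollingGuard_2's Aiming and Shooting with sensing success.
; A sensed actor is written to the blackboard enemy key, which is cleared when sensing fails.
; Storing the last seen location is disconnected, and a debug print helper is unused.
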(event `self.ReceiveBeginPlay`
  (bind _blackboardcomponent (`self.UseBlackboard` "/Game/Dynamic/NPC/AI/PatrolData.PatrolData"))
  (set `self.BlackboardComp` _blackboardcomponent)
  (`self.RunBehaviorTree` "/Game/Dynamic/NPC/AI/GuardBehaviour.GuardBehaviour"))

(event `self.AIPerception.OnTargetPerceptionUpdated`
  (params (Actor :type "Actor Object Reference") (Stimulus :type "AIStimulus Structure"))
  (bind _enemykey (`self.EnemyKey`))
  (bind _blackboardcomp (`self.BlackboardComp`))
  (if (not (`self.ActorHasTag` Actor "Enemy"))
    (bind _aspatrolling_guard_2 (cast `/Game/Dynamic/NPC/Behaviour/PatrollingGuard_2` (`self.K2_GetPawn`)))
    (bind _output_get (set `/Game/Dynamic/NPC/Behaviour/PatrollingGuard_2.Aiming` (`.bSuccessfullySensed` (break `AIStimulus` Stimulus)) _aspatrolling_guard_2))
    (bind _output_get_2 (set `/Game/Dynamic/NPC/Behaviour/PatrollingGuard_2.Shooting` _output_get _aspatrolling_guard_2))
    (if _output_get_2
      (`BlackboardComponent.SetValueAsObject` _blackboardcomp _enemykey Actor)
      (else
        (`BlackboardComponent.ClearValue` _blackboardcomp _enemykey)))))

(fn `Print Stimulus`
  (params (Object :type "Object Object Reference") (Class :type "Object Class Reference"))
  (`KismetSystemLibrary.PrintString` (`KismetStringLibrary.Concat_StrStr` (`KismetSystemLibrary.GetObjectName` (`self.K2_GetPawn`)) " " (`KismetSystemLibrary.GetClassDisplayName` Class) " " (`KismetSystemLibrary.GetObjectName` Object))))

(fn `UserConstructionScript`)